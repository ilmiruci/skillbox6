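; BP_BALL is a ball actor that moves in a straight line and bounces off whatever it hits.
; Each tick it applies a swept world offset along Direction at Speed, and on a blocking hit reflects Direction around the surface normal.
; Every bounce also subtracts a fixed amount, a fraction of the starting Speed cached at BeginPlay, never dropping below MinSpeed.
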(event EventBeginPlay
  (Variables|Default|SetPercentation (* (Variables|Default|GetSpeed) 0.1)))

(event Collision|EventActorBeginOverlap
  (params (OtherActor :type Actor%20Object%20Reference)))

(event EventTick
  (params (DeltaSeconds :type Float%20%28single-precision%29))
  (bind _sweephitresult (Transformation|AddActorWorldOffset (* (* (Variables|Default|GetDirection%20) (Variables|Default|GetSpeed)) DeltaSeconds) true))
  (if (.bBlockingHit (Collision|BreakHitResult _sweephitresult))
    (Variables|Default|SetDirection%20 (Math|Vector|GetReflectionVector (Variables|Default|GetDirection%20) (.Normal (Collision|BreakHitResult _sweephitresult))))
    (Variables|Default|SetSpeed (Math|Float|Max(Float) (- (Variables|Default|GetSpeed) (Variables|Default|GetPercentation)) (Variables|Default|GetMinSpeed)))))

(fn ConstructionScript)